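; BP_Ratna01 is a damage actor whose Sphere hurts actors that enter it.
; Sphere begin overlap prints the other actor's first tag and applies fixed damage if it differs from the Instigator's first tag, crediting the Instigator.
; A looping-timer Damage event is disconnected; its loop over overlapping actors damages the overlap event's OtherActor rather than each element, without a tag check.
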(event OnComponentBeginOverlap(Sphere)
  (params (OverlappedComponent :type Primitive%20Component%20Object%20Reference) (OtherActor :type Actor%20Object%20Reference) (OtherComp :type Primitive%20Component%20Object%20Reference) (OtherBodyIndex :type Integer) (bFromSweep :type Boolean) (SweepResult :type Hit%20Result%20Structure%20%28by%20ref%29))
  (bind _tags (Variables|/Script/Engine.Actor|GetTags OtherActor))
  (bind _output (Utilities|Array|Get(acopy) _tags))
  (if (!= OtherActor self)
    (Development|PrintString (Utilities|String|ToString(Name) _output))
    (if (!= _output (Utilities|Array|Get(acopy) (Variables|/Script/Engine.Actor|GetTags (Game|GetInstigator))))
      (Game|Damage|ApplyDamage OtherActor 1e+02 0 (Game|GetInstigator)))))

(event Custom|Damage
  (for _array_element (Collision|GetOverlappingActors (Variables|Default|GetSphere) 0 :!class /Script/Engine.PrimitiveComponent)
    (Game|Damage|ApplyDamage (stale OnComponentBeginOverlap(Sphere) OtherActor) 1e+02 0 (Game|GetInstigator))))

(event EventBeginPlay)

(event Collision|EventActorBeginOverlap
  (params (OtherActor :type Actor%20Object%20Reference)))

(event EventTick
  (params (DeltaSeconds :type Float%20%28single-precision%29)))

(fn ConstructionScript)