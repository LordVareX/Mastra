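; Base character Blueprint with a team, a level and an overhead health/mana widget, plus team-based map icon visibility.
; BeginPlay tags the actor with its team name and hides the widget icon, while events push health and level stats into that widget.
; Sphere overlap reveals enemy map icons, but leaving only hides this character's widget icon.
; Multi sets all characters' icons by team; its only call is disconnected, among other leftover nodes.
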(event OnComponentBeginOverlap(Sphere)
  (params (OverlappedComponent :type Primitive%20Component%20Object%20Reference) (OtherActor :type Actor%20Object%20Reference) (OtherComp :type Primitive%20Component%20Object%20Reference) (OtherBodyIndex :type Integer) (bFromSweep :type Boolean) (SweepResult :type Hit%20Result%20Structure%20%28by%20ref%29))
  (Development|PrintString "In")
  (if (!= OtherActor self)
    (bind _asbp_base_character (Utilities|Casting|CastToBP_BaseCharacter OtherActor))
    (if (!= (Variables|/Script/Mastra.MastraCharacter|GetTeam _asbp_base_character) (Variables|Default|GetTeam))
      (Class|MapIconComponent|SetIconVisible (Variables|BP_BaseCharacter_C|GetMapIcon _asbp_base_character) true))))

(event OnComponentEndOverlap(Sphere)
  (params (OverlappedComponent :type Primitive%20Component%20Object%20Reference) (OtherActor :type Actor%20Object%20Reference) (OtherComp :type Primitive%20Component%20Object%20Reference) (OtherBodyIndex :type Integer))
  (Development|PrintString "out")
  (if (!= OtherActor self)
    (bind _asw_health_mana (Utilities|Casting|CastToW_HealthMana (UserInterface|GetWidget (Variables|Default|GetWidget))))
    (Default|HideIcon _asw_health_mana)))

(event Custom|AddLevel
  (CallFunction|ClientAddLevel))

(event Custom|Multi
  (bind _outactors (Actor|GetAllActorsOfClass "BP_BaseCharacter_C"))
  (for _array_element _outactors
    (Development|PrintString (Utilities|String|ToString(Integer) (Variables|/Script/Mastra.MastraCharacter|GetTeam _array_element)))
    (if (== (Variables|/Script/Mastra.MastraCharacter|GetTeam _array_element) (Variables|Default|GetTeam))
      (Class|MapIconComponent|SetIconVisible (Variables|BP_BaseCharacter_C|GetMapIcon _array_element) false)
      (else
        (Class|MapIconComponent|SetIconVisible (Variables|BP_BaseCharacter_C|GetMapIcon _array_element) true)))))

(event Custom|ClientAddLevel
  (bind _result (Math|Integer|IncrementInt (Variables|Default|GetLevel))
    (:%20%20
      (Variables|Default|SetLevel _result)
      (Class|MastraCharacter|ServerLevelIncreased (Variables|Default|GetPickedCharacter)))))

(event Custom|serverrep
  (params (PC :type Player%20Controller%20Object%20Reference)))

(event EventUpdateUI
  (params (currentHealth :type Float%20%28single-precision%29))
  (bind _asw_health_mana (Utilities|Casting|CastToW_HealthMana (UserInterface|GetWidget (Variables|Default|GetWidget))))
  (Variables|/Game/Gary/Widgets/W_HealthMana.W_HealthMana_C|SetHP _asw_health_mana currentHealth))

(event EventBeginPlay
  (bind _teamname (Variables|Default|GetTeamName))
  (Development|PrintString (Utilities|String|Append "Team : " (Utilities|String|ToString(Name) _teamname)))
  (Utilities|Array|SetArrayElem (Variables|Default|GetTags) 0 _teamname)
  (bind _asw_health_mana (Utilities|Casting|CastToW_HealthMana (UserInterface|GetWidget (Variables|Default|GetWidget))))
  (Default|HideIcon _asw_health_mana))

(event EventUpdateStats
  (params (currMaxHealth :type Float%20%28single-precision%29) (currLevel :type Integer))
  (bind _asw_health_mana (Utilities|Casting|CastToW_HealthMana (UserInterface|GetWidget (Variables|Default|GetWidget))))
  (Variables|/Game/Gary/Widgets/W_HealthMana.W_HealthMana_C|SetMaxHP _asw_health_mana currMaxHealth)
  (Variables|/Game/Gary/Widgets/W_HealthMana.W_HealthMana_C|SetLevel _asw_health_mana currLevel))

(fn ConstructionScript)