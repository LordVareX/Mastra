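; Base MOBA unit character that takes commands, fights, recalls, and on death grants exp and gold to its killer.
; Authority turns high-level commands into Move/Attack micro-commands run through AIMoveTo, with attack-move engaging perceived enemies and idle or recalling units retaliating when damaged.
; Components handle HP/MP, level-scaled params, targeting, sight and events; params drive regen and speeds.
; Tick updates the status widget and shows or hides the unit by the local team's vision.
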(event Custom|SetCommand
  (params (Command :type Command%20Enum :default "NewEnumerator0") (TargetLocation :type Vector) (TargetUnit :type Unit%20Object%20Reference))
  ;[1 1 1] SetCommand
  (bind _alive (CallFunction|IsAlive))
  (if (and _alive (Variables|Server|GetCanCommand))
    (CallFunction|ResetCommand)
    (bind _output_get (Variables|Server|SetCommand Command))
    (switch Utilities|FlowControl|Switch|SwitchonCommand _output_get
      (:NewEnumerator1
        (CallFunction|SetMicroCommand "NewEnumerator1" TargetLocation :!label _label))
      (:NewEnumerator2
        (CallFunction|SetMicroCommand "NewEnumerator2" "0, 0, 0" TargetUnit))
      (:NewEnumerator3
        (goto _label)))))

(event Custom|Init
  (params (UnitKey :type Name) (Team :type Team%20Enum :default "NewEnumerator0") (PlayerState :type My%20Player%20State%20Object%20Reference) (OwnerUnit :type Unit%20Object%20Reference))
  ;[1 1 1] Init
  (Variables|Client&Server|SetUnitKey UnitKey)
  (Variables|Client&Server|SetTeam Team)
  (Variables|Client&Server|SetCommanderPlayerState PlayerState)
  (Variables|Server|SetOwnerUnit OwnerUnit)
  (EventDispatchers|BindEventtoOnResetTargetEventDispatcher (Variables|Default|GetTargetComponent) (EventDispatchers|CreateEvent :!event Custom|OnResetTarget))
  (bind _returnvalue (Utilities|GetDataTableRow "/Game/OpenMoba/DataTables/UnitDataTable.UnitDataTable" (Variables|Client&Server|GetUnitKey))
    (:then
      (Variables|Server|SetUnitRadius (.UnitRadius (Utilities|Struct|BreakUnitData _returnvalue))))))

(event Custom|SetMicroCommand
  (params (MicroCommand :type MicroCommand%20Enum :default "NewEnumerator0") (Location :type Vector) (Unit :type Unit%20Object%20Reference))
  ;[1 1 1] SetMicroCommand
  (CallFunction|StopMovement)
  (switch Utilities|FlowControl|Switch|SwitchonMicroCommand MicroCommand
    (:NewEnumerator1
      (Variables|Client&Server|SetAnimState "NewEnumerator1")
      (Variables|Server|SetMicroCommand "NewEnumerator1")
      (bind _output_get (Variables|Server|SetTargetLocation Location))
      (AI|AIMoveTo (AI|GetAIController self) _output_get 0 -1.0 "Default" "Default" true true))
    (:NewEnumerator2
      (Variables|Client&Server|SetAnimState "NewEnumerator1")
      (Variables|Server|SetMicroCommand "NewEnumerator2")
      (Default|SetTarget (Variables|Default|GetTargetComponent) Unit)
      (AI|AIMoveTo (AI|GetAIController self) "0, 0, 0" Unit -1.0 "Default" "Default" true true))))

(event Custom|OnResetTarget
  ;[1 1 1] OnResetTarget
  (CallFunction|StopMovement)
  (Variables|Client&Server|SetAnimState "NewEnumerator0")
  (Variables|Server|SetMicroCommand "NewEnumerator0"))

(event Custom|AddExpGold
  (params (Exp :type Float%20%28single-precision%29) (Gold :type Integer))
  (bind _returnvalue (Actor|GetComponentbyClass "/Game/OpenMoba/Blueprints/Components/InventoryComponent.InventoryComponent_C"))
  ;[1 1 1] AddExpGold
  (Default|AddExp (Variables|Default|GetLevelComponent) Exp)
  (Utilities|IsValid _returnvalue
    (:Is%20Valid
      (Default|AddGold _returnvalue Gold))))

(event EventBeginPlay
  (bind _returnvalue (Game|GetPlayerController 0))
  ;[1 1 1] BeginPlay
  (Utilities|IsValid _returnvalue
    (:Is%20Valid
      (bind _returnvalue_2 (UserInterface|CreateWidget "/Game/OpenMoba/Blueprints/Widgets/UnitStatusWidget.UnitStatusWidget_C" _returnvalue))
      (bind _output_get (Variables|Client|SetHud _returnvalue_2))
      (UserInterface|Viewport|AddtoViewport _output_get 0)
      (Networking|SwitchHasAuthority
        (:Authority
          (Timeline|Regen Play
            (:Regen
              (bind _alive (CallFunction|IsAlive))
              (if _alive
                (Utilities|FlowControl|Sequence
                  (:then_0
                    (bind _value (CallFunction|GetUnitParam "NewEnumerator2"))
                    (bind _value_2 (CallFunction|GetUnitParam "NewEnumerator0"))
                    (Default|AddHP (Variables|Default|GetHPMPComponent) (* _value_2 _value)))
                  (:then_1
                    (bind _value_3 (CallFunction|GetUnitParam "NewEnumerator3"))
                    (bind _value_4 (CallFunction|GetUnitParam "NewEnumerator1"))
                    (Default|AddMP (Variables|Default|GetHPMPComponent) (* _value_4 _value_3))))))))))))

(event Collision|EventActorBeginOverlap
  (params (OtherActor :type Actor%20Object%20Reference)))

(event EventDispatchByteEvent
  (params (ByteEvent :type ByteEvent%20Enum :default "NewEnumerator0") (Arg :type Byte :default 0))
  ;[1 1 1] DispatchByteEvent
  (Default|DispatchByteEvent (Variables|Default|GetEventComponent) ByteEvent Arg))

(event Game|Damage|EventAnyDamage
  (params (Damage :type Float%20%28single-precision%29) (DamageType :type Damage%20Type%20Object%20Reference) (InstigatedBy :type Controller%20Object%20Reference) (DamageCauser :type Actor%20Object%20Reference))
  ;[1 1 1] AnyDamage
  (bind _alive (CallFunction|IsAlive))
  (if _alive
    (Default|AddHP (Variables|Default|GetHPMPComponent) (- 0.0 Damage))
    (bind _alive_2 (CallFunction|IsAlive))
    (if _alive_2
      (switch Utilities|FlowControl|Switch|SwitchonCommand (Variables|Server|GetCommand)
        (:NewEnumerator0
          _)
        (:NewEnumerator4
          _))
      (bind _asunit (Utilities|Casting|CastToUnit DamageCauser))
      (CallFunction|SetCommand "NewEnumerator2" "0, 0, 0" _asunit)
      (else
        (Utilities|FlowControl|Sequence
          (:then_0
            (bind _exp (CallFunction|GetExp))
            (bind _gold (CallFunction|GetGold))
            (bind _asunit_2 (Utilities|Casting|CastToUnit DamageCauser))
            (CallFunction|AddExpGold _asunit_2 _exp _gold))
          (:then_1
            (CallFunction|ResetCommand)
            (Variables|Client&Server|SetAnimState "NewEnumerator3")
            (CallFunction|DispatchNormalEvent "NewEnumerator0")))))))

(event EventDispatchNormalEvent
  (params (NormalEvent :type NormalEvent%20Enum :default "NewEnumerator0"))
  ;[1 1 1] DispatchNormalEvent
  (Default|DispatchNormalEvent (Variables|Default|GetEventComponent) NormalEvent))

(event EventTick
  (params (DeltaSeconds :type Float%20%28single-precision%29))
  (bind _returnvalue (Game|GetPlayerController 0))
  (bind _hud (Variables|Client|GetHud))
  ;[1 1 1] Tick
  (Utilities|FlowControl|Sequence
    (:then_0
      (Utilities|IsValid _returnvalue
        (:Is%20Valid
          (bind _asmy_player_state (Utilities|Casting|CastToMyPlayerState (Variables|/Script/Engine.Controller|GetPlayerState _returnvalue)))
          (bind _vision (CallFunction|GetVision (Variables|/Game/OpenMoba/Blueprints/PlayerState/MyPlayerState.MyPlayerState_C|GetTeam _asmy_player_state)))
          (CallFunction|SetAppearance _vision))))
    (:then_1
      (Utilities|IsValid _hud
        (:Is%20Valid
          (Default|UpdateStatus _hud self))))
    (:then_2
      (bind _value (CallFunction|GetUnitParam "NewEnumerator8"))
      (Variables|Client&Server|SetAttackSpeed _value))
    (:then_3
      (Networking|SwitchHasAuthority
        (:Authority
          (Utilities|FlowControl|Sequence
            (:then_0
              (Collision|SetCollisionResponsetoChannel (Variables|Collision|GetCapsuleComponent) "ECC_Pawn" (select (Variables|Server|GetCollisionEnabled) "ECR_Block" "ECR_Ignore")))
            (:then_1
              (bind _value_2 (CallFunction|GetUnitParam "NewEnumerator9"))
              (Variables|/Script/Engine.CharacterMovementComponent|SetMaxWalkSpeed (Variables|Character|GetCharacterMovement) _value_2))
            (:then_2
              (Utilities|UpdateCommand))
            (:then_3
              (Utilities|UpdateMicroCommand))))))))

(event EventSetAppearance
  (params (Vision :type Vision%20Enum :default "NewEnumerator0"))
  (bind _returnvalue (Utilities|Select :Index Vision :NewEnumerator0 true :NewEnumerator1 true :NewEnumerator2 false))
  ;[1 1 1] SetAppearance
  (Rendering|SetVisibility (Variables|Character|GetMesh) _returnvalue true)
  (bind _alive (CallFunction|IsAlive))
  (Widget|SetVisibility (Variables|Client|GetHud) (select (and _alive _returnvalue) "Visible" "Hidden")))

(event EventEndPlay
  (params (EndPlayReason :type EEndPlayReason%20Enum :default "Destroyed"))
  (bind _hud (Variables|Client|GetHud))
  ;[1 1 1] EndPlay
  (Utilities|IsValid _hud
    (:Is%20Valid
      (Widget|RemovefromParent _hud))))

(fn ConstructionScript)

(fn GetOwnerUnit
  (Utilities|IsValid (Variables|Server|GetOwnerUnit)
    (:Is%20Valid
      (return (Variables|Server|GetOwnerUnit)))
    (:Is%20Not%20Valid
      (return self))))

(fn GetUnitParam
  (params (Param :type Param%20Enum :default "NewEnumerator0"))
  (bind _levelcomponent (Variables|Default|GetLevelComponent))
  (bind _addvalue (Default|GetAddParam _levelcomponent Param))
  (bind _mulvalue (Default|GetMulParam _levelcomponent Param))
  (return (* _mulvalue _addvalue)))

(fn OnRepUnitKey
  (Default|Init (Variables|Default|GetLevelComponent)))

(fn ResetCommand
  (Variables|Server|SetCommand "NewEnumerator0")
  (Default|ResetTarget (Variables|Default|GetTargetComponent))
  (Variables|Server|SetRecallTimer 0.0))

(fn StopMovement
  (Components|Movement|StopMovementImmediately (Variables|Character|GetCharacterMovement)))

(fn GetAnimState
  (return (Variables|Client&Server|GetAnimState)))

(fn GetByteEventDispatcher
  (params (ByteEvent :type ByteEvent%20Enum :default "NewEnumerator0"))
  (bind _wrapper (Default|GetByteEventDispatcher (Variables|Default|GetEventComponent) ByteEvent))
  (return _wrapper))

(fn GetCommanderPlayerState
  (return (Variables|Client&Server|GetCommanderPlayerState)))

(fn GetExp
  (return 0.0))

(fn GetGold
  (return 0))

(fn GetNormalEventDispatcher
  (params (NormalEvent :type NormalEvent%20Enum :default "NewEnumerator0"))
  (bind _wrapper (Default|GetNormalEventDispatcher (Variables|Default|GetEventComponent) NormalEvent))
  (return _wrapper))

(fn GetVision
  (params (Team :type Team%20Enum :default "NewEnumerator0"))
  (bind _visible (Default|GetSight (Variables|Default|GetSightComponent) Team))
  (return (select (and _visible (Variables|Server|GetVisible)) "NewEnumerator0" "NewEnumerator2")))

(fn IsAlive
  (bind _alive (Default|IsAlive (Variables|Default|GetHPMPComponent)))
  (return _alive))