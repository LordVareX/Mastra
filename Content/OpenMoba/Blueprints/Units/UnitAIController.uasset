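; AI controller for OpenMoba units that supplies target queries built on AI perception.
; GetPerceivedUnits merges sight and damage senses into a unique list of units on other teams, optionally only living ones.
; GetNearestAlivePerceivedUnit picks the closest living one to the controlled pawn, optionally excluding one team (yellow, per the parameter name), and reports whether any was found.
; The event graph holds no active logic.
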(event EventBeginPlay)

(event EventTick
  (params (DeltaSeconds :type Float%20%28single-precision%29)))

(fn ConstructionScript)

(fn GetPerceivedUnits
  (params (Alive :type Boolean))
  (LocalVariables|SetLocalAlive Alive)
  (Utilities|FlowControl|Sequence
    (:then_0
      (if (LocalVariables|GetLocalAlive)
        (for _array_element (Class|AIPerceptionComponent|GetCurrentlyPerceivedActors (Variables|Default|GetAIPerception) "/Script/AIModule.AISense_Sight")
          (bind _asunit (Utilities|Casting|CastToUnit _array_element))
          (bind _output_get (LocalVariables|SetLocalUnit _asunit))
          (bind _team (Utilities|GetOwnerTeam)
            (:Get
              (bind _alive (Default|IsAlive (LocalVariables|GetLocalUnit)))
              (if (and _alive (Utilities|Enum|NotEqual(Enum) _team (Variables|/Game/OpenMoba/Blueprints/Units/Unit.Unit_C|GetTeam _output_get)))
                (Utilities|Array|AddUnique (LocalVariables|GetRetUnits) (LocalVariables|GetLocalUnit))))))
        (else
          (for _array_element_2 (Class|AIPerceptionComponent|GetCurrentlyPerceivedActors (Variables|Default|GetAIPerception) "/Script/AIModule.AISense_Sight")
            (bind _asunit_2 (Utilities|Casting|CastToUnit _array_element_2))
            (bind _output_get_2 (LocalVariables|SetLocalUnit _asunit_2))
            (bind _team_2 (Utilities|GetOwnerTeam)
              (:Get
                (if (Utilities|Enum|NotEqual(Enum) _team_2 (Variables|/Game/OpenMoba/Blueprints/Units/Unit.Unit_C|GetTeam _output_get_2))
                  (Utilities|Array|AddUnique (LocalVariables|GetRetUnits) (LocalVariables|GetLocalUnit)))))))))
    (:then_1
      (if (LocalVariables|GetLocalAlive)
        (for _array_element_3 (Class|AIPerceptionComponent|GetCurrentlyPerceivedActors (Variables|Default|GetAIPerception) "/Script/AIModule.AISense_Damage")
          (bind _asunit_3 (Utilities|Casting|CastToUnit _array_element_3))
          (bind _output_get_3 (LocalVariables|SetLocalUnit _asunit_3))
          (bind _team_3 (Utilities|GetOwnerTeam)
            (:Get
              (bind _alive_2 (Default|IsAlive (LocalVariables|GetLocalUnit)))
              (if (and _alive_2 (Utilities|Enum|NotEqual(Enum) _team_3 (Variables|/Game/OpenMoba/Blueprints/Units/Unit.Unit_C|GetTeam _output_get_3)))
                (Utilities|Array|AddUnique (LocalVariables|GetRetUnits) (LocalVariables|GetLocalUnit))))))
        (else
          (for _array_element_4 (Class|AIPerceptionComponent|GetCurrentlyPerceivedActors (Variables|Default|GetAIPerception) "/Script/AIModule.AISense_Damage")
            (bind _asunit_4 (Utilities|Casting|CastToUnit _array_element_4))
            (bind _output_get_4 (LocalVariables|SetLocalUnit _asunit_4))
            (bind _team_4 (Utilities|GetOwnerTeam)
              (:Get
                (if (Utilities|Enum|NotEqual(Enum) _team_4 (Variables|/Game/OpenMoba/Blueprints/Units/Unit.Unit_C|GetTeam _output_get_4))
                  (Utilities|Array|AddUnique (LocalVariables|GetRetUnits) (LocalVariables|GetLocalUnit)))))))))
    (:then_2
      (return (LocalVariables|GetRetUnits)))))

(fn GetNearestAlivePerceivedUnit
  (params (ContainYellowTeamUnit :type Boolean))
  (bind _localunits (LocalVariables|GetLocalUnits))
  (bind _output (Utilities|Array|Get(acopy) _localunits))
  (if ContainYellowTeamUnit
    (bind _units (CallFunction|GetPerceivedUnits true))
    (Utilities|Array|AppendArray (LocalVariables|GetLocalUnits) _units)
    (else
      (bind _units_2 (CallFunction|GetPerceivedUnits true))
      (for _array_element _units_2
        (if (Utilities|Enum|NotEqual(Enum) (Variables|/Game/OpenMoba/Blueprints/Units/Unit.Unit_C|GetTeam _array_element) "NewEnumerator0")
          (Utilities|Array|Add (LocalVariables|GetLocalUnits) _array_element)))))
  (if (> (Utilities|Array|Length (LocalVariables|GetLocalUnits)) 0)
    (bind _asunit (Utilities|Casting|CastToUnit (Pawn|GetControlledPawn)))
    (bind _output_get (LocalVariables|SetOwnerUnit _asunit))
    (bind _distance (CallFunction|GetUnitDistance _output_get _output))
    (LocalVariables|SetNearestUnit _output)
    (LocalVariables|SetDistance _distance)
    (for _array_element_2 (LocalVariables|GetLocalUnits)
      (bind _distance_2 (CallFunction|GetUnitDistance _array_element_2 (LocalVariables|GetOwnerUnit)))
      (if (< _distance_2 (LocalVariables|GetDistance))
        (LocalVariables|SetNearestUnit _array_element_2)
        (LocalVariables|SetDistance _distance_2)))
    (return (LocalVariables|GetNearestUnit) true)
    (else
      (return 0 false))))