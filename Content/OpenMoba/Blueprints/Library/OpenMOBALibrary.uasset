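; OpenMOBALibrary is a Blueprint function library of spatial helpers for the OpenMoba game.
; GetSymmetryTransform mirrors a transform through the world origin in X and Y and negates yaw, keeping height, roll, pitch and scale.
; GetUnitDistance and GetUnitGroundDistance measure flat XY distance between two units or from a unit to a point, subtracting unit radii to give edge-based gaps.
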(fn GetSymmetryTransform
  (params (Transform :type Transform))
  (bind (_location _rotation _scale) (Math|Transform|BreakTransform Transform))
  (bind (_x _y _z) (Math|Vector|BreakVector _location))
  (bind (_roll _pitch _yaw) (Math|Rotator|BreakRotator _rotation))
  (return (Math|Transform|MakeTransform (Math|Vector|MakeVector (- 0.0 _x) (- 0.0 _y) _z) (Math|Rotator|MakeRotator _roll _pitch (- 0.0 _yaw)) _scale)))

(fn GetUnitDistance
  (params (Unit0 :type Unit%20Object%20Reference) (Unit1 :type Unit%20Object%20Reference))
  (bind _returnvalue (Transformation|GetActorLocation Unit1))
  (bind _returnvalue_2 (Transformation|GetActorLocation Unit0))
  (bind (_x _y) (Math|Vector|BreakVector _returnvalue))
  (bind (_x_2 _y_2) (Math|Vector|BreakVector _returnvalue_2))
  (return (- (Math|Vector|VectorLength (- (Math|Vector|MakeVector _x_2 _y_2 0.0) (Math|Vector|MakeVector _x _y 0.0))) (+ (Variables|/Game/OpenMoba/Blueprints/Units/Unit.Unit_C|GetUnitRadius Unit0) (Variables|/Game/OpenMoba/Blueprints/Units/Unit.Unit_C|GetUnitRadius Unit1)))))

(fn GetUnitGroundDistance
  (params (Unit :type Unit%20Object%20Reference) (Ground :type Vector))
  (bind (_x _y) (Math|Vector|BreakVector Ground))
  (bind _returnvalue (Transformation|GetActorLocation Unit))
  (bind (_x_2 _y_2) (Math|Vector|BreakVector _returnvalue))
  (return (- (Math|Vector|VectorLength (- (Math|Vector|MakeVector _x_2 _y_2 0.0) (Math|Vector|MakeVector _x _y 0.0))) (Variables|/Game/OpenMoba/Blueprints/Units/Unit.Unit_C|GetUnitRadius Unit))))