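; Fog of war actor that reveals areas around units on the local player's team using a fog render target.
; Each tick it clears the target to black, then filters all units by team and vision state relative to the player's CommandUnit.
; A short downward trace at a fixed height over each qualifying unit yields a collision UV.
; That UV feeds a dynamic subtract-fog material, which is drawn into the render target.
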(event Custom|DrawSubtract
  (params (LocationtoDraw :type Vector%202D%20Structure))
  ;[1 1 1] DrawSubtract
  (Rendering|Material|SetVectorParameterValue (Variables|Default|GetMaterialInstance) "DrawLocation" (Math|Conversions|ToLinearColor(Vector) (Math|Conversions|ToVector(Vector2D) LocationtoDraw)) :!class /Script/Engine.MaterialInstanceDynamic)
  (Rendering|DrawMaterialtoRenderTarget "/Game/OpenMoba/Blueprints/FogOfWar/FogTextureRenderTarget.FogTextureRenderTarget" (Variables|Default|GetMaterialInstance)))

(event EventBeginPlay
  ;[1 1 1] BeginPlay
  (bind _returnvalue (Rendering|Material|CreateDynamicMaterialInstance "/Game/OpenMoba/Blueprints/FogOfWar/SubtractFogMaterial.SubtractFogMaterial" "None" "None" :!class /Script/Engine.KismetMaterialLibrary))
  (Variables|Default|SetMaterialInstance _returnvalue)
  (Rendering|ClearRenderTarget2D "/Game/OpenMoba/Blueprints/FogOfWar/FogTextureRenderTarget.FogTextureRenderTarget")
  (Rendering|SetVisibility (Variables|Default|GetPlane) true false))

(event Collision|EventActorBeginOverlap
  (params (OtherActor :type Actor%20Object%20Reference)))

(event EventTick
  (params (DeltaSeconds :type Float%20%28single-precision%29))
  ;[1 1 1] Tick
  (bind _asmy_player_controller (Utilities|Casting|CastToMyPlayerController (Game|GetPlayerController 0)))
  (Utilities|IsValid (Variables|/Game/OpenMoba/Blueprints/PlayerController/MyPlayerController.MyPlayerController_C|GetCommandUnit _asmy_player_controller)
    (:Is%20Valid
      (Rendering|ClearRenderTarget2D "/Game/OpenMoba/Blueprints/FogOfWar/FogTextureRenderTarget.FogTextureRenderTarget")
      (bind _outactors (Actor|GetAllActorsOfClass "/Game/OpenMoba/Blueprints/Units/Unit.Unit_C"))
      (for _array_element _outactors
        (bind _vision (Default|GetVision _array_element (Variables|/Game/OpenMoba/Blueprints/Units/Unit.Unit_C|GetTeam (Variables|/Game/OpenMoba/Blueprints/PlayerController/MyPlayerController.MyPlayerController_C|GetCommandUnit _asmy_player_controller))))
        (if (and (Utilities|Enum|NotEqual(Enum) _vision "NewEnumerator2") (Utilities|Enum|Equal(Enum) (Variables|/Game/OpenMoba/Blueprints/Units/Unit.Unit_C|GetTeam _array_element) (Variables|/Game/OpenMoba/Blueprints/Units/Unit.Unit_C|GetTeam (Variables|/Game/OpenMoba/Blueprints/PlayerController/MyPlayerController.MyPlayerController_C|GetCommandUnit _asmy_player_controller))))
          (bind (_outhit _returnvalue) (Collision|LineTraceByChannel (Math|Vector|MakeVector (.X (Math|Vector|BreakVector (Transformation|GetActorLocation _array_element))) (.Y (Math|Vector|BreakVector (Transformation|GetActorLocation _array_element))) 2.1e+02) (+ (Math|Vector|MakeVector (.X (Math|Vector|BreakVector (Transformation|GetActorLocation _array_element))) (.Y (Math|Vector|BreakVector (Transformation|GetActorLocation _array_element))) 2.1e+02) "0.000000, 0,-20.000000") "TraceTypeQuery5" true 0 "None" false))
          (if _returnvalue
            (CallFunction|DrawSubtract (.UV (Class|GameplayStatics|FindCollisionUV _outhit)))))))))

(fn ConstructionScript)