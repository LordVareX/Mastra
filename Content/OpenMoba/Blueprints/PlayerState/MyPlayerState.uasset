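; Player state for a MOBA that holds each player's custom name, team, champion key and ready flag.
; SetPlayerState updates only changed values, then has MyGameMode change the team or champion, or run a ready check as needed.
; RepNotify handlers for the replicated fields refresh the local scoreboard through MyPlayerController at player index 0.
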(event Custom|SetPlayerState
  (params (CustomeName :type String) (Team :type Team%20Enum :default "NewEnumerator0") (ChampionKeyName :type Name) (Ready :type Boolean))
  ;[1 1 1] SetPlayerState
  (Utilities|FlowControl|Sequence
    (:then_0
      (if (Utilities|Enum|NotEqual(Enum) (Variables|Default|GetCustomeName) CustomeName)
        (Variables|Default|SetCustomeName CustomeName)))
    (:then_1
      (if (Utilities|Enum|NotEqual(Enum) (Variables|Default|GetTeam) Team)
        (bind _output_get (Variables|Default|SetTeam Team))
        (bind _asmy_game_mode (Utilities|Casting|CastToMyGameMode (Game|GetGameMode)))
        (Default|ChangeTeam _asmy_game_mode (Variables|Default|GetPlayerController) _output_get)))
    (:then_2
      (if (Utilities|Name|NotEqual(Name) (Variables|Default|GetChampionKey) ChampionKeyName)
        (bind _output_get_2 (Variables|Default|SetChampionKey ChampionKeyName))
        (bind _asmy_game_mode_2 (Utilities|Casting|CastToMyGameMode (Game|GetGameMode)))
        (Default|ChangeChampion _asmy_game_mode_2 (Variables|Default|GetPlayerController) _output_get_2)))
    (:then_3
      (if (Math|Boolean|NotEqual(Boolean) (Variables|Default|GetReady) Ready)
        (Variables|Default|SetReady Ready)
        (bind _asmy_game_mode_3 (Utilities|Casting|CastToMyGameMode (Game|GetGameMode)))
        (Default|RedyCheck _asmy_game_mode_3)))))

(event EventBeginPlay)

(event EventTick
  (params (DeltaSeconds :type Float%20%28single-precision%29)))

(fn ConstructionScript)

(fn OnRepCustomeName
  (bind _asmy_player_controller (Utilities|Casting|CastToMyPlayerController (Game|GetPlayerController 0)))
  (Default|UpdateScoreboard _asmy_player_controller))

(fn OnRepTeam
  (bind _asmy_player_controller (Utilities|Casting|CastToMyPlayerController (Game|GetPlayerController 0)))
  (Default|UpdateScoreboard _asmy_player_controller))

(fn OnRepChampionKeyName
  (bind _asmy_player_controller (Utilities|Casting|CastToMyPlayerController (Game|GetPlayerController 0)))
  (Default|UpdateScoreboard _asmy_player_controller))

(fn OnRepReady
  (bind _asmy_player_controller (Utilities|Casting|CastToMyPlayerController (Game|GetPlayerController 0)))
  (Default|UpdateScoreboard _asmy_player_controller))