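; Game mode for a MOBA match, managing player spawning, team and champion changes, recall, and battle flow.
; First login maps fountains by team and initializes the UnitFactory and MinionSpawner; joining players alternate teams and receive a default champion.
; All players readying starts battle, opening fountains and enabling minion spawns.
; Nexus death announces victory, disables units and, after a delay, resets the match by respawning units and champions.
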(event Custom|ResetGame
  ;[1 1 1] ResetGame
  (Utilities|OpenFountain false)
  (Default|DestroyAllUnits (Variables|Default|GetUnitFactory))
  (Utilities|SpawnTargetPointUnitsandSetEventtoNexus
    (:Set
      (bind _myplayerstate (Utilities|GetAllMyPlayerState)
        (:LoopBody
          (bind _transform (CallFunction|GetSpawnTransform (Variables|/Game/OpenMoba/Blueprints/PlayerState/MyPlayerState.MyPlayerState_C|GetTeam _myplayerstate)))
          (Default|SpawnUnit (Variables|Default|GetUnitFactory) (Variables|/Game/OpenMoba/Blueprints/PlayerState/MyPlayerState.MyPlayerState_C|GetTeam _myplayerstate) (Variables|/Game/OpenMoba/Blueprints/PlayerState/MyPlayerState.MyPlayerState_C|GetChampionKey _myplayerstate) _transform "AdjustIfPossibleButAlwaysSpawn" (Variables|/Game/OpenMoba/Blueprints/PlayerState/MyPlayerState.MyPlayerState_C|GetPlayerController _myplayerstate))
          (Variables|/Game/OpenMoba/Blueprints/PlayerState/MyPlayerState.MyPlayerState_C|SetReady _myplayerstate false))))))

(event Custom|SetBattleState
  (params (NewBattleState :type BattleState%20Enum :default "NewEnumerator0"))
  ;[1 1 1] SetBattleState
  (bind _asmy_game_state (Utilities|Casting|CastToMyGameState (Game|GetGameState)))
  (bind _output_get (Variables|/Game/OpenMoba/Blueprints/GameState/MyGameState.MyGameState_C|SetBattleState _asmy_game_state NewBattleState))
  (switch Utilities|FlowControl|Switch|SwitchonBattleState _output_get
    (:NewEnumerator0
      (CallFunction|ResetGame)
      (CallFunction|SetCenterTexttoAllClient "Prepare for Battle" 96 (Utilities|Struct|MakeSlateColor "(R=1.000000,G=1.000000,B=1.000000,A=1.000000)") 4.0))
    (:NewEnumerator1
      (Utilities|OpenFountain true)
      (Default|SetSpawn (Variables|Default|GetMinionSpawner) true)
      (CallFunction|SetCenterTexttoAllClient "Battle Start" 96 (Utilities|Struct|MakeSlateColor "(R=1.000000,G=1.000000,B=1.000000,A=1.000000)") 4.0))
    (:NewEnumerator2
      (Default|DisableAllUnits (Variables|Default|GetUnitFactory))
      (Default|SetSpawn (Variables|Default|GetMinionSpawner) false))))

(event Custom|RedyCheck
  (bind _returnvalue (Game|GetGameState))
  (bind _playerarray (Variables|/Script/Engine.GameStateBase|GetPlayerArray _returnvalue))
  ;[1 1 1] RedyCheck
  (bind _battlestate (Utilities|GetBattleState)
    (:Get
      (if (and (Utilities|Enum|Equal(Enum) _battlestate "NewEnumerator0") (> (Utilities|Array|Length _playerarray) 0))
        (Variables|Default|SetAllReady true)
        (bind _array_element (Utilities|Array|ForEachLoopwithBreak _playerarray :!label _label)
          (:LoopBody
            (bind _asmy_player_state (Utilities|Casting|CastToMyPlayerState _array_element))
            (if (not (Variables|/Game/OpenMoba/Blueprints/PlayerState/MyPlayerState.MyPlayerState_C|GetReady _asmy_player_state))
              (Variables|Default|SetAllReady false)
              (goto _label Break)))
          (:Completed
            (if (Variables|Default|GetAllReady)
              (CallFunction|SetBattleState "NewEnumerator1"))))))))

(event Custom|Init
  ;[1 1 1] Init
  (Utilities|FlowControl|Sequence
    (:then_0
      (bind _outactors (Actor|GetAllActorsOfClass "/Game/OpenMoba/Blueprints/Fountain/Fountain.Fountain_C"))
      (for _array_element _outactors
        (Utilities|Map|Add (Variables|Default|GetFountains) (Variables|/Game/OpenMoba/Blueprints/Fountain/Fountain.Fountain_C|GetTeam _array_element) _array_element)
        (Default|SetOpen _array_element false)))
    (:then_1
      (Utilities|IsValid (Variables|Default|GetUnitFactory)
        (:Is%20Valid
          _)
        (:Is%20Not%20Valid
          (bind _returnvalue (Game|SpawnActorfromClass "/Game/OpenMoba/Blueprints/GameMode/UnitFactory/UnitFactory.UnitFactory_C" (Math|Transform|MakeTransform "0, 0, 0") "AlwaysSpawn" 0 0))))
      (bind _output_get (Variables|Default|SetUnitFactory _returnvalue))
      (Default|Init _output_get))
    (:then_2
      (Utilities|IsValid (Variables|Default|GetMinionSpawner)
        (:Is%20Valid
          _)
        (:Is%20Not%20Valid
          (bind _returnvalue_2 (Game|SpawnActorfromClass "/Game/OpenMoba/Blueprints/GameMode/MinionSpawner/MinionSpawner.MinionSpawner_C" (Math|Transform|MakeTransform "0, 0, 0") "AlwaysSpawn" 0 0))))
      (bind _output_get_2 (Variables|Default|SetMinionSpawner _returnvalue_2))
      (Default|Init _output_get_2 (Variables|Default|GetUnitFactory))
      (Default|SetSpawn _output_get_2 false))
    (:then_3
      (Utilities|SpawnTargetPointUnitsandSetEventtoNexus))))

(event Custom|ChangeChampion
  (params (PlayerController :type Player%20Controller%20Object%20Reference) (ChampionKeyName :type Name))
  ;[1 1 1] ChangeChampion
  (bind _asmy_player_controller (Utilities|Casting|CastToMyPlayerController PlayerController))
  (bind _output_get (Variables|Default|SetPreviousTeam (Variables|/Game/OpenMoba/Blueprints/Units/Unit.Unit_C|GetTeam (Variables|/Game/OpenMoba/Blueprints/PlayerController/MyPlayerController.MyPlayerController_C|GetCommandUnit _asmy_player_controller))))
  (Actor|DestroyActor (Variables|/Game/OpenMoba/Blueprints/PlayerController/MyPlayerController.MyPlayerController_C|GetCommandUnit _asmy_player_controller))
  (bind _transform (CallFunction|GetSpawnTransform _output_get))
  (Default|SpawnUnit (Variables|Default|GetUnitFactory) (Variables|Default|GetPreviousTeam) ChampionKeyName _transform "AdjustIfPossibleButAlwaysSpawn" PlayerController))

(event Custom|RecallUnit
  (params (Unit :type Unit%20Object%20Reference))
  ;[1 1 1] RecallUnit
  (bind _transform (CallFunction|GetSpawnTransform (Variables|/Game/OpenMoba/Blueprints/Units/Unit.Unit_C|GetTeam Unit)))
  (Transformation|SetActorTransform Unit _transform))

(event Custom|SetNexusDeathEvent
  ;[1 1 1] SetNexusDeathEvent
  (bind _outactors (Actor|GetAllActorsOfClass "/Game/OpenMoba/Blueprints/Units/ImmobileUnit/Nexus/Nexus.Nexus_C"))
  (for _array_element _outactors
    (bind _wrapper (Default|GetNormalEventDispatcher _array_element "NewEnumerator0"))
    (EventDispatchers|BindEventtoWrappedEventDispatcher _wrapper (delegate Custom|OnDeath))))

(event Custom|OnDeath
  (params (Actor :type Actor%20Object%20Reference))
  ;[1 1 1] SetNexusDeathEvent
  (bind _asunit (Utilities|Casting|CastToUnit Actor))
  (CallFunction|SetCenterTexttoAllClient "Victory" 128 (select (Utilities|Enum|Equal(Enum) (Variables|/Game/OpenMoba/Blueprints/Units/Unit.Unit_C|GetTeam _asunit) "NewEnumerator2") (Utilities|Struct|MakeSlateColor "(R=0.000000,G=0.000000,B=1.000000,A=1.000000)") (Utilities|Struct|MakeSlateColor "(R=1.000000,G=0.000000,B=0.000000,A=1.000000)")) (- (Variables|Default|GetRestartGameTime) 1.0))
  (bind _battlestate (Utilities|GetBattleState)
    (:Get
      (if (Utilities|Enum|NotEqual(Enum) _battlestate "NewEnumerator2")
        (CallFunction|SetBattleState "NewEnumerator2")
        (Utilities|FlowControl|Delay (Variables|Default|GetRestartGameTime))
        (CallFunction|SetBattleState "NewEnumerator0")))))

(event Custom|ChangeTeam
  (params (PlayerController :type Player%20Controller%20Object%20Reference) (Team :type Team%20Enum :default "NewEnumerator0"))
  ;[1 1 1] ChangeTeam
  (bind _asmy_player_controller (Utilities|Casting|CastToMyPlayerController PlayerController))
  (Variables|Default|SetPreviousChampionKey (Variables|/Game/OpenMoba/Blueprints/Units/Unit.Unit_C|GetUnitKey (Variables|/Game/OpenMoba/Blueprints/PlayerController/MyPlayerController.MyPlayerController_C|GetCommandUnit _asmy_player_controller)))
  (Actor|DestroyActor (Variables|/Game/OpenMoba/Blueprints/PlayerController/MyPlayerController.MyPlayerController_C|GetCommandUnit _asmy_player_controller))
  (bind _transform (CallFunction|GetSpawnTransform Team))
  (Default|SpawnUnit (Variables|Default|GetUnitFactory) Team (Variables|Default|GetPreviousChampionKey) _transform "AdjustIfPossibleButAlwaysSpawn" PlayerController))

(event Custom|SetCenterTextToAllClient
  (params (Text :type Text) (FontSize :type Integer) (Color :type Slate%20Color%20Structure) (Duration :type Float%20%28double-precision%29))
  ;[1 1 1] SetCenterTextToAllClient
  (bind _myplayerstate (Utilities|GetAllMyPlayerState)
    (:LoopBody
      (bind _asmy_player_controller (Utilities|Casting|CastToMyPlayerController (Variables|/Game/OpenMoba/Blueprints/PlayerState/MyPlayerState.MyPlayerState_C|GetPlayerController _myplayerstate)))
      (Default|SetCenterTextWidget _asmy_player_controller Text FontSize Color Duration))))

(event EventBeginPlay)

(event EventTick
  (params (DeltaSeconds :type Float%20%28single-precision%29)))

(event EventPostLogin
  (params (NewPlayer :type Player%20Controller%20Object%20Reference))
  ;[1 1 1] OnPostLogin
  (if (not (Variables|Default|GetInitFlag))
    (Variables|Default|SetInitFlag true)
    (CallFunction|Init))
  (bind _output_get (Variables|Default|SetNewPlayer NewPlayer))
  (bind _asmy_player_controller (Utilities|Casting|CastToMyPlayerController _output_get))
  (Default|Init _asmy_player_controller)
  (Utilities|FlowControl|FlipFlop
    (:A
      (Variables|Default|SetSpawnTeam "NewEnumerator1"))
    (:B
      (Variables|Default|SetSpawnTeam "NewEnumerator2")))
  (bind _transform (CallFunction|GetSpawnTransform (Variables|Default|GetSpawnTeam)))
  (Default|SpawnUnit (Variables|Default|GetUnitFactory) (Variables|Default|GetSpawnTeam) (Variables|Default|GetDefaultChampionKey) _transform "AdjustIfPossibleButAlwaysSpawn" (Variables|Default|GetNewPlayer))
  (bind _playerstate (CallFunction|GetPlayerState (Variables|Default|GetNewPlayer)))
  (CallFunction|SetPlayerState (Variables|Default|GetNewPlayer) (Variables|/Game/OpenMoba/Blueprints/PlayerState/MyPlayerState.MyPlayerState_C|GetCustomeName _playerstate) (Variables|Default|GetSpawnTeam) (Variables|Default|GetDefaultChampionKey) false))

(event EventOnLogout
  (params (ExitingController :type Controller%20Object%20Reference))
  ;[1 1 1] OnLogout
  (bind _asmy_player_controller (Utilities|Casting|CastToMyPlayerController ExitingController))
  (Utilities|IsValid (Variables|/Game/OpenMoba/Blueprints/PlayerController/MyPlayerController.MyPlayerController_C|GetCommandUnit _asmy_player_controller)
    (:Is%20Valid
      (Actor|DestroyActor (Variables|/Game/OpenMoba/Blueprints/PlayerController/MyPlayerController.MyPlayerController_C|GetCommandUnit _asmy_player_controller)))))

(fn ConstructionScript)

(fn SetPlayerState
  (params (PlayerController :type Player%20Controller%20Object%20Reference) (CustomeName :type String) (Team :type Team%20Enum :default "NewEnumerator0") (ChampionKeyName :type Name) (Ready :type Boolean))
  (bind _asmy_player_state (Utilities|Casting|CastToMyPlayerState (Variables|/Script/Engine.Controller|GetPlayerState PlayerController)))
  (Utilities|FlowControl|Sequence
    (:then_0
      (Variables|/Game/OpenMoba/Blueprints/PlayerState/MyPlayerState.MyPlayerState_C|SetPlayerController _asmy_player_state PlayerController))
    (:then_1
      (Variables|/Game/OpenMoba/Blueprints/PlayerState/MyPlayerState.MyPlayerState_C|SetCustomeName _asmy_player_state CustomeName))
    (:then_2
      (Variables|/Game/OpenMoba/Blueprints/PlayerState/MyPlayerState.MyPlayerState_C|SetTeam _asmy_player_state Team))
    (:then_3
      (Variables|/Game/OpenMoba/Blueprints/PlayerState/MyPlayerState.MyPlayerState_C|SetChampionKey _asmy_player_state ChampionKeyName))
    (:then_4
      (Variables|/Game/OpenMoba/Blueprints/PlayerState/MyPlayerState.MyPlayerState_C|SetReady _asmy_player_state Ready))))

(fn GetPlayerState
  (params (PlayerController :type Player%20Controller%20Object%20Reference))
  (bind _asmy_player_state (Utilities|Casting|CastToMyPlayerState (Variables|/Script/Engine.Controller|GetPlayerState PlayerController)))
  (return _asmy_player_state))

(fn GetSpawnTransform
  (params (Team :type Team%20Enum :default "NewEnumerator0"))
  (bind _fountains (Variables|Default|GetFountains))
  (bind _value (Utilities|Map|Find _fountains Team))
  (Utilities|IsValid _value
    (:Is%20Valid
      (bind _transform (Default|GetSpawnTransform _value))
      (return _transform))))