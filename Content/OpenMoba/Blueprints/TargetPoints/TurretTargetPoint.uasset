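; TurretTargetPoint is a Blueprint target point for turrets in OpenMoba, tagged with a Blue or Red team.
; Its construction script switches on Team and applies the matching blue or red material to its Sphere component, so the team shows on placed instances.
; The event graph holds only disabled default events, so it adds no runtime logic of its own.
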(event EventBeginPlay
  (|CallParentFunction) ; This node is disabled and will not be called.\nDrag off pins to build functionality.
)

(event Collision|EventActorBeginOverlap
  (params (OtherActor :type Actor%20Object%20Reference))
  (|CallParentFunction OtherActor) ; This node is disabled and will not be called.\nDrag off pins to build functionality.
)

(event EventTick
  (params (DeltaSeconds :type Float%20%28single-precision%29))
  (|CallParentFunction DeltaSeconds) ; This node is disabled and will not be called.\nDrag off pins to build functionality.
)

(fn ConstructionScript
  (bind _sphere (Variables|Default|GetSphere))
  (|CallParentFunction)
  (switch Utilities|FlowControl|Switch|SwitchonTeam (Variables|Default|GetTeam)
    (:NewEnumerator1
      (Rendering|Material|SetMaterial _sphere 0 "/Game/OpenMoba/Materials/BlueMaterial.BlueMaterial"))
    (:NewEnumerator2
      (Rendering|Material|SetMaterial _sphere 0 "/Game/OpenMoba/Materials/RedMaterial.RedMaterial"))))