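; Target component that stores a unit's current target in OpenMoba and exposes it through GetTargetUnit.
; SetTarget binds to two normal and one byte wrapped event dispatcher on the target unit.
; ResetTarget broadcasts OnResetTarget, then unbinds those dispatchers and clears the target if it is valid.
; HideTarget triggers that reset when the passed team matches the owning unit's team.
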(event Custom|SetTarget
  (params (Unit :type Unit%20Object%20Reference))
  ;[1 1 1] SetTarget
  (Variables|Default|SetUnit Unit)
  (Utilities|FlowControl|Sequence
    (:then_0
      (bind _wrapper (Default|GetNormalEventDispatcher (Variables|Default|GetUnit) "NewEnumerator0"))
      (EventDispatchers|BindEventtoWrappedEventDispatcher _wrapper (EventDispatchers|CreateEvent :!event Custom|ResetTarget)))
    (:then_1
      (bind _wrapper_2 (Default|GetNormalEventDispatcher (Variables|Default|GetUnit) "NewEnumerator1"))
      (EventDispatchers|BindEventtoWrappedEventDispatcher _wrapper_2 (EventDispatchers|CreateEvent :!event Custom|ResetTarget)))
    (:then_2
      (bind _wrapper_3 (Default|GetByteEventDispatcher (Variables|Default|GetUnit) "NewEnumerator0"))
      (EventDispatchers|BindEventtoWrappedEventDispatcher _wrapper_3 (EventDispatchers|CreateEvent :!event Custom|HideTarget)))))

(event Custom|HideTarget
  (params (Actor :type Actor%20Object%20Reference) (Team :type Byte))
  ;[1 1 1] HideTarget
  (bind _asunit (Utilities|Casting|CastToUnit (Components|GetOwner)))
  (if (== (Variables|/Game/OpenMoba/Blueprints/Units/Unit.Unit_C|GetTeam _asunit) Team)
    (CallFunction|ResetTarget Actor)))

(event Custom|ResetTarget
  (params (Actor :type Actor%20Object%20Reference))
  ;[1 1 1] ResetTarget
  (Default|CallOnResetTargetEventDispatcher)
  (Utilities|IsValid (Variables|Default|GetUnit)
    (:Is%20Valid
      (Utilities|FlowControl|Sequence
        (:then_0
          (bind _wrapper (Default|GetNormalEventDispatcher (Variables|Default|GetUnit) "NewEnumerator0"))
          (EventDispatchers|UnbindEventfromWrappedEventDispatcher _wrapper (EventDispatchers|CreateEvent :!event Custom|ResetTarget)))
        (:then_1
          (bind _wrapper_2 (Default|GetNormalEventDispatcher (Variables|Default|GetUnit) "NewEnumerator1"))
          (EventDispatchers|UnbindEventfromWrappedEventDispatcher _wrapper_2 (EventDispatchers|CreateEvent :!event Custom|ResetTarget)))
        (:then_2
          (bind _wrapper_3 (Default|GetByteEventDispatcher (Variables|Default|GetUnit) "NewEnumerator0"))
          (EventDispatchers|UnbindEventfromWrappedEventDispatcher _wrapper_3 (EventDispatchers|CreateEvent :!event Custom|HideTarget)))
        (:then_3
          (Variables|Default|SetUnit 0))))))

(event EventBeginPlay)

(event EventTick
  (params (DeltaSeconds :type Float%20%28single-precision%29)))

(fn GetTargetUnit
  (return (Variables|Default|GetUnit)))