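; Inventory component for a MOBA unit that holds gold and a fixed set of item slots.
; Slots store ItemDataTable row keys, with EmptyItemKey marking free ones; AddItem fills the first free slot.
; Consume spawns the row's ConsumeItemClass as a temporary actor, applies it to the owning Unit, destroys it and clears the slot.
; GetAddParam and GetMulParam combine held items' additive and multiplicative bonuses for a requested stat.
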(event Custom|AddGold
  (params (Gold :type Integer))
  ;[1 1 1] AddGold
  (Variables|Client&Server|SetGold (+ Gold (Variables|Client&Server|GetGold))))

(event Custom|Consume
  (params (Index :type Integer))
  (bind _itemkeys (Variables|Client&Server|GetItemKeys))
  (bind _output (Utilities|Array|Get(acopy) _itemkeys Index))
  ;[1 1 1] Consume
  (bind _returnvalue (Utilities|GetDataTableRow "/Game/OpenMoba/DataTables/ItemDataTable.ItemDataTable" _output)
    (:then
      (if (Utilities|IsValidClass (.ConsumeItemClass (Utilities|Struct|BreakItemData _returnvalue)))
        (bind _returnvalue_2 (Game|SpawnActorfromClass (.ConsumeItemClass (Utilities|Struct|BreakItemData _returnvalue)) (Math|Transform|MakeTransform "0, 0, 0") "AlwaysSpawn" 0 0))
        (bind _asunit (Utilities|Casting|CastToUnit (Components|GetOwner)))
        (Default|Consume _returnvalue_2 _asunit _output)
        (Actor|DestroyActor _returnvalue_2)
        (CallFunction|RemoveItem Index)))))

(event Custom|RemoveItem
  (params (Index :type Integer))
  ;[1 1 1] RemoveItem
  (Utilities|Array|SetArrayElem (Variables|Client&Server|GetItemKeys) Index (Variables|Client&Server|GetEmptyItemKey)))

(event Custom|AddItem
  (params (ItemKey :type Name))
  ;[1 1 1] AddItem
  (bind (_found _index) (CallFunction|GetEmptySlot))
  (if _found
    (Utilities|GetDataTableRow "/Game/OpenMoba/DataTables/ItemDataTable.ItemDataTable" ItemKey
      (:then
        (Utilities|Array|SetArrayElem (Variables|Client&Server|GetItemKeys) _index ItemKey)))))

(event EventBeginPlay)

(event EventTick
  (params (DeltaSeconds :type Float%20%28single-precision%29)))

(fn GetItem
  (params (Index :type Integer))
  (bind _maxnum (CallFunction|GetMaxItemNum))
  (if (< Index _maxnum)
    (return (Utilities|Array|Get(acopy) (Variables|Client&Server|GetItemKeys) Index))
    (else
      (return (Variables|Client&Server|GetEmptyItemKey)))))

(fn GetEmptySlot
  (for (_array_element _array_index) (Variables|Client&Server|GetItemKeys)
    (if (Utilities|Name|Equal(Name) _array_element (Variables|Client&Server|GetEmptyItemKey))
      (return true _array_index)))
  (return false 0))

(fn GetMaxItemNum
  (return (Utilities|Array|Length (Variables|Client&Server|GetItemKeys))))

(fn GetAddParam
  (params (Param :type Param%20Enum :default "NewEnumerator0"))
  (for _array_element (Variables|Client&Server|GetItemKeys)
    (if (Utilities|Name|NotEqual(Name) _array_element (Variables|Client&Server|GetEmptyItemKey))
      (bind _returnvalue (Utilities|GetDataTableRow "/Game/OpenMoba/DataTables/ItemDataTable.ItemDataTable" _array_element)
        (:then
          (LocalVariables|SetSum (+ (LocalVariables|GetSum) (Utilities|Select :Index Param :NewEnumerator0 (.AddHP (Utilities|Struct|BreakItemData _returnvalue)) :NewEnumerator1 (.AddMP (Utilities|Struct|BreakItemData _returnvalue)) :NewEnumerator2 (.AddHPRegen (Utilities|Struct|BreakItemData _returnvalue)) :NewEnumerator3 (.AddMPRegen (Utilities|Struct|BreakItemData _returnvalue)) :NewEnumerator4 (.AddMeleeAttack (Utilities|Struct|BreakItemData _returnvalue)) :NewEnumerator5 (.AddMagicPower (Utilities|Struct|BreakItemData _returnvalue)) :NewEnumerator6 (.AddDefence (Utilities|Struct|BreakItemData _returnvalue)) :NewEnumerator7 (.AddMagicResist (Utilities|Struct|BreakItemData _returnvalue)) :NewEnumerator8 (.AddAttackSpeed (Utilities|Struct|BreakItemData _returnvalue)) :NewEnumerator10 (.AddAttackRange (Utilities|Struct|BreakItemData _returnvalue)) :NewEnumerator9 (.AddMovementSpeed (Utilities|Struct|BreakItemData _returnvalue)))))))))
  (return (LocalVariables|GetSum)))

(fn GetMulParam
  (params (Param :type Param%20Enum :default "NewEnumerator0"))
  (for _array_element (Variables|Client&Server|GetItemKeys)
    (if (Utilities|Name|NotEqual(Name) _array_element (Variables|Client&Server|GetEmptyItemKey))
      (bind _returnvalue (Utilities|GetDataTableRow "/Game/OpenMoba/DataTables/ItemDataTable.ItemDataTable" _array_element)
        (:then
          (LocalVariables|SetSum (* (LocalVariables|GetSum) (Utilities|Select :Index Param :NewEnumerator0 (.MulHP (Utilities|Struct|BreakItemData _returnvalue)) :NewEnumerator1 (.MulMP (Utilities|Struct|BreakItemData _returnvalue)) :NewEnumerator2 (.MulHPRegen (Utilities|Struct|BreakItemData _returnvalue)) :NewEnumerator3 (.MulMPRegen (Utilities|Struct|BreakItemData _returnvalue)) :NewEnumerator4 (.MulMeleeAttack (Utilities|Struct|BreakItemData _returnvalue)) :NewEnumerator5 (.MulMagicPower (Utilities|Struct|BreakItemData _returnvalue)) :NewEnumerator6 (.MulDefence (Utilities|Struct|BreakItemData _returnvalue)) :NewEnumerator7 (.MulMagicResist (Utilities|Struct|BreakItemData _returnvalue)) :NewEnumerator8 (.MulAttackSpeed (Utilities|Struct|BreakItemData _returnvalue)) :NewEnumerator10 (.MulAttackRange (Utilities|Struct|BreakItemData _returnvalue)) :NewEnumerator9 (.MulMovementSpeed (Utilities|Struct|BreakItemData _returnvalue)))))))))
  (return (LocalVariables|GetSum)))