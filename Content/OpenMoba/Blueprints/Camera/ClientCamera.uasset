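; Client-side MOBA camera actor that makes itself the local player's view target on BeginPlay and either follows an actor or pans freely.
; Each Tick it lerps toward the followed actor in auto-follow mode, otherwise it snaps to a stored focus location.
; Scrolling or setting a focus location turns auto-follow off, and a separate event re-enables it.
; Zoom slides the camera component along a fixed diagonal offset within clamped limits.
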(event Custom|Scroll
  (params (Vector :type Vector))
  ;[1 1 1] Scroll
  (Variables|Default|SetFocusLocation (+ (* Vector (Utilities|Time|GetWorldDeltaSeconds)) (Variables|Default|GetFocusLocation)))
  (Variables|Default|SetAutoFollow false))

(event Custom|SetFocusLocation
  (params (Target :type Vector))
  ;[1 1 1] SetFocusLocation
  (Variables|Default|SetFocusLocation Target)
  (Variables|Default|SetAutoFollow false))

(event Custom|Init
  (params (Actor :type Actor%20Object%20Reference))
  ;[1 1 1] Init
  (Variables|Default|SetFollowActor Actor))

(event Custom|Zoom
  (params (Amount :type Float%20%28single-precision%29))
  ;[1 1 1] Zoom
  (bind _output_get (Variables|Default|SetCurZoom (Math|Float|Clamp(Float) (+ (* Amount (Variables|Default|GetZoomSpeed)) (Variables|Default|GetCurZoom)) (Variables|Default|GetMinZoom) (Variables|Default|GetMaxZoom))))
  (Transformation|SetRelativeLocation (Variables|Default|GetCamera) (* "-1.000000,0.000000,1.000000" _output_get) false false))

(event Custom|AutoFollowActor
  ;[1 1 1] AutoFollowActor
  (Variables|Default|SetAutoFollow true))

(event EventBeginPlay
  (bind _returnvalue (Game|GetPlayerController 0))
  ;[1 1 1] BeginPlay
  (Utilities|IsValid _returnvalue
    (:Is%20Valid
      (Game|Player|SetViewTargetwithBlend _returnvalue self 0.0 "VTBlend_Linear" 0.0 false))))

(event Collision|EventActorBeginOverlap
  (params (OtherActor :type Actor%20Object%20Reference)))

(event EventTick
  (params (DeltaSeconds :type Float%20%28single-precision%29))
  ;[1 1 1] Tick
  (Utilities|IsValid (Variables|Default|GetFollowActor)
    (:Is%20Valid
      (if (Variables|Default|GetAutoFollow)
        (Transformation|SetActorLocation (Math|Vector|Lerp(Vector) (Transformation|GetActorLocation) (Transformation|GetActorLocation (Variables|Default|GetFollowActor)) (* DeltaSeconds 6.0)) false false)
        (Variables|Default|SetFocusLocation (Transformation|GetActorLocation))
        (else
          (Transformation|SetActorLocation (Variables|Default|GetFocusLocation) false false))))))

(fn ConstructionScript)