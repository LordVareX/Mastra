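; MOBA player controller that turns input into orders for its replicated CommandUnit and manages camera and UI.
; Mouse traces choose attack on visible living enemies, move or attack-move, passed through Send events to SetCommand.
; It also validates lobby player state and handles item use, selling and fountain-range purchases.
; CommandUnit's OnRep creates the local ClientCamera for scroll, zoom, follow and minimap jumps, while widgets route through MyGameInstance.
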(event Custom|SendConsumeItem
  (params (Index :type Integer))
  ;[1 1 1] SendConsumeItem
  (if (Utilities|IsCommandUnitValid)
    (bind _aschampion (Utilities|Casting|CastToChampion (Variables|Client&Server|GetCommandUnit)))
    (Default|Consume (Variables|/Game/OpenMoba/Blueprints/Units/MobileUnit/Champions/Champion.Champion_C|GetInventoryComponent _aschampion) Index)))

(event Custom|SellItem
  (params (Index :type Integer))
  ;[1 1 1] SellItem
  (if (Utilities|IsCommandUnitValid)
    (bind _aschampion (Utilities|Casting|CastToChampion (Variables|Client&Server|GetCommandUnit)))
    (bind _itemkey (Default|GetItem (Variables|/Game/OpenMoba/Blueprints/Units/MobileUnit/Champions/Champion.Champion_C|GetInventoryComponent _aschampion) Index))
    (if (Utilities|Name|NotEqual(Name) _itemkey (Variables|/Game/OpenMoba/Blueprints/Components/InventoryComponent.InventoryComponent_C|GetEmptyItemKey (Variables|/Game/OpenMoba/Blueprints/Units/MobileUnit/Champions/Champion.Champion_C|GetInventoryComponent _aschampion)))
      (bind _returnvalue (Utilities|GetDataTableRow "/Game/OpenMoba/DataTables/ItemDataTable.ItemDataTable" _itemkey)
        (:then
          (Default|RemoveItem (Variables|/Game/OpenMoba/Blueprints/Units/MobileUnit/Champions/Champion.Champion_C|GetInventoryComponent _aschampion) Index)
          (Default|AddGold (Variables|/Game/OpenMoba/Blueprints/Units/MobileUnit/Champions/Champion.Champion_C|GetInventoryComponent _aschampion) (.SellPrice (Utilities|Struct|BreakItemData _returnvalue))))))))

(event Custom|SendAttack
  (params (TargetUnit :type Unit%20Object%20Reference))
  ;[1 1 1] SendAttack
  (Default|SetCommand (Variables|Client&Server|GetCommandUnit) "NewEnumerator2" "0, 0, 0" TargetUnit))

(event Custom|ReceivePlayerState
  (params (CustomeName :type String) (Team :type Team%20Enum :default "NewEnumerator0") (ChampionKeyName :type Name) (Ready :type Boolean))
  ;[1 1 1] ReceivePlayerState
  (bind _asmy_game_state (Utilities|Casting|CastToMyGameState (Game|GetGameState)))
  (if (Utilities|Enum|NotEqual(Enum) (Variables|/Game/OpenMoba/Blueprints/GameState/MyGameState.MyGameState_C|GetBattleState _asmy_game_state) "NewEnumerator2")
    (if (and (> (Utilities|String|Len CustomeName) 0) (Utilities|Enum|NotEqual(Enum) Team "NewEnumerator0"))
      (Utilities|GetDataTableRow "/Game/OpenMoba/DataTables/UnitDataTable.UnitDataTable" ChampionKeyName
        (:then
          (bind _asmy_player_state (Utilities|Casting|CastToMyPlayerState (Variables|GetPlayerState)))
          (Default|SetPlayerState _asmy_player_state CustomeName Team ChampionKeyName Ready))))))

(event Custom|SendRecallCommand
  ;[1 1 1] SendRecallCommand
  (Default|SetCommand (Variables|Client&Server|GetCommandUnit) "NewEnumerator4" "0, 0, 0"))

(event Custom|BuyItem
  (params (ItemKey :type Name))
  ;[1 1 1] BuyItem
  (if (Utilities|IsCommandUnitValid)
    (bind _aschampion (Utilities|Casting|CastToChampion (Variables|Client&Server|GetCommandUnit)))
    (bind _outactors (Actor|GetAllActorsOfClass "/Game/OpenMoba/Blueprints/Fountain/Fountain.Fountain_C"))
    (for _array_element _outactors
      (if (Utilities|Enum|Equal(Enum) (Variables|/Game/OpenMoba/Blueprints/Fountain/Fountain.Fountain_C|GetTeam _array_element) (Variables|/Game/OpenMoba/Blueprints/Units/Unit.Unit_C|GetTeam (Variables|Client&Server|GetCommandUnit)))
        (bind _distance (CallFunction|GetUnitGroundDistance (Variables|Client&Server|GetCommandUnit) (Transformation|GetActorLocation _array_element)))
        (if (<= _distance 1e+03)
          (bind _returnvalue (Utilities|GetDataTableRow "/Game/OpenMoba/DataTables/ItemDataTable.ItemDataTable" ItemKey)
            (:then
              (bind _found (Default|GetEmptySlot (Variables|/Game/OpenMoba/Blueprints/Units/MobileUnit/Champions/Champion.Champion_C|GetInventoryComponent _aschampion)))
              (if (and _found (>= (Variables|/Game/OpenMoba/Blueprints/Components/InventoryComponent.InventoryComponent_C|GetGold (Variables|/Game/OpenMoba/Blueprints/Units/MobileUnit/Champions/Champion.Champion_C|GetInventoryComponent _aschampion)) (.BuyPrice (Utilities|Struct|BreakItemData _returnvalue))))
                (Default|AddGold (Variables|/Game/OpenMoba/Blueprints/Units/MobileUnit/Champions/Champion.Champion_C|GetInventoryComponent _aschampion) (- 0 (.BuyPrice (Utilities|Struct|BreakItemData _returnvalue))))
                (Default|AddItem (Variables|/Game/OpenMoba/Blueprints/Units/MobileUnit/Champions/Champion.Champion_C|GetInventoryComponent _aschampion) ItemKey)))))))))

(event Custom|ClickMiniMap
  (params (Location :type Vector%202D%20Structure))
  (bind (_x _y) (Math|Vector2D|BreakVector2D Location))
  ;[1 1 1] ClickMiniMap
  (Default|SetFocusLocation (Variables|Client|GetClientCamera) (Math|Vector|MakeVector (* _y 5e+03) (* _x 5e+03) 0.0)))

(event Custom|SendIdleCommand
  ;[1 1 1] SendIdleCommand
  (Default|SetCommand (Variables|Client&Server|GetCommandUnit) "NewEnumerator0" "0, 0, 0"))

(event Custom|SendPlayerState
  (params (CustomeName :type String) (Team :type Team%20Enum :default "NewEnumerator0") (ChampionKeyName :type Name) (Ready :type Boolean))
  ;[1 1 1] SendPlayerState
  (CallFunction|ReceivePlayerState CustomeName Team ChampionKeyName Ready))

(event Custom|OpenShopWidget
  ;[1 1 1] Shop
  (bind _visible (CallFunction|IsWidgetVisible "/Game/OpenMoba/Blueprints/Widgets/ScoreboardWidget.ScoreboardWidget_C"))
  (if _visible
    (CallFunction|RemoveWidget "/Game/OpenMoba/Blueprints/Widgets/ScoreboardWidget.ScoreboardWidget_C")
    (CallFunction|AddWidget "/Game/OpenMoba/Blueprints/Widgets/Shop/ShopWidget.ShopWidget_C" 2)
    (else
      (bind _visible_2 (CallFunction|IsWidgetVisible "/Game/OpenMoba/Blueprints/Widgets/Shop/ShopWidget.ShopWidget_C"))
      (if _visible_2
        (CallFunction|RemoveWidget "/Game/OpenMoba/Blueprints/Widgets/Shop/ShopWidget.ShopWidget_C")
        (else
          (CallFunction|AddWidget "/Game/OpenMoba/Blueprints/Widgets/Shop/ShopWidget.ShopWidget_C" 2))))))

(event Custom|SetCenterTextWidget
  (params (CenterText :type Text) (FontSize :type Integer) (Color :type Slate%20Color%20Structure) (Duration :type Float%20%28single-precision%29))
  ;[1 1 1] SetCenterTextWidget
  (bind _widget (CallFunction|AddWidget "/Game/OpenMoba/Blueprints/Widgets/CenterTextWidget.CenterTextWidget_C" 3))
  (bind _ascenter_text_widget (Utilities|Casting|CastToCenterTextWidget _widget))
  (Default|SetCenterText _ascenter_text_widget CenterText FontSize Color)
  (Utilities|FlowControl|Delay Duration)
  (CallFunction|RemoveWidget "/Game/OpenMoba/Blueprints/Widgets/CenterTextWidget.CenterTextWidget_C"))

(event Custom|UpdateScoreboard
  ;[1 1 1] UpdateScoreboard
  (bind _visible (CallFunction|IsWidgetVisible "/Game/OpenMoba/Blueprints/Widgets/ScoreboardWidget.ScoreboardWidget_C"))
  (if _visible
    (bind _widget (CallFunction|GetWidget "/Game/OpenMoba/Blueprints/Widgets/ScoreboardWidget.ScoreboardWidget_C"))
    (bind _asscoreboard_widget (Utilities|Casting|CastToScoreboardWidget _widget))
    (Default|UpdatePlayerStates _asscoreboard_widget)))

(event Custom|SendAttackMove
  (params (GoalLocation :type Vector))
  ;[1 1 1] SendAttackMove
  (Default|SetCommand (Variables|Client&Server|GetCommandUnit) "NewEnumerator3" GoalLocation))

(event Custom|Init
  ;[1 1 1] Init
  (CallFunction|AddWidget "/Game/OpenMoba/Blueprints/Widgets/CommandUnitStatusWidget.CommandUnitStatusWidget_C" 1)
  (CallFunction|AddWidget "/Game/OpenMoba/Blueprints/Widgets/MiniMapWidget.MiniMapWidget_C" 1)
  (Input|SetInputModeGameandUI self 0 "DoNotLock" true)
  (Variables|Default|SetbShowMouseCursor true))

(event Custom|SendMoveCommand
  (params (GroundLocation :type Vector))
  ;[1 1 1] SendMoveCommand
  (Default|SetCommand (Variables|Client&Server|GetCommandUnit) "NewEnumerator1" GroundLocation))

(event EventBeginPlay)

(event EventTick
  (params (DeltaSeconds :type Float%20%28single-precision%29))
  ;[1 1 1] Tick
  (CallFunction|ScrollCamera))

(event Input|ActionEvents|InputActionRecall
  (params (Key :type Key%20Structure))
  ;[1 1 1] Recall
  (:Pressed
    (if (Utilities|IsCommandUnitValid)
      (CallFunction|SendRecallCommand))))

(event Input|ActionEvents|InputActionMiddleMouseButtonDown
  (params (Key :type Key%20Structure))
  (bind (_worldlocation _worlddirection) (Game|Player|ConvertMouseLocationToWorldSpace))
  ;[1 1 1] MiddleMouseButtonDown
  (:Pressed
    (if (Utilities|IsCommandUnitValid)
      (bind (_outhit _returnvalue) (Collision|LineTraceByChannel _worldlocation (+ _worldlocation (* _worlddirection 1e+04)) "TraceTypeQuery3" false 0 "None"))
      (if _returnvalue
        (CallFunction|SendAttackMove (.Location (Collision|BreakHitResult _outhit)))))))

(event Input|ActionEvents|InputActionConsumeItem0
  (params (Key :type Key%20Structure))
  ;[1 1 1] ConsumeItem
  (:Pressed
    (CallFunction|SendConsumeItem)))

(event Input|ActionEvents|InputActionScoreboard
  (params (Key :type Key%20Structure))
  ;[1 1 1] Scoreboard
  (:Pressed
    (bind _visible (CallFunction|IsWidgetVisible "/Game/OpenMoba/Blueprints/Widgets/Shop/ShopWidget.ShopWidget_C"))
    (if _visible
      (CallFunction|RemoveWidget "/Game/OpenMoba/Blueprints/Widgets/Shop/ShopWidget.ShopWidget_C")
      (CallFunction|AddWidget "/Game/OpenMoba/Blueprints/Widgets/ScoreboardWidget.ScoreboardWidget_C" 2)
      (else
        (bind _visible_2 (CallFunction|IsWidgetVisible "/Game/OpenMoba/Blueprints/Widgets/ScoreboardWidget.ScoreboardWidget_C"))
        (if _visible_2
          (CallFunction|RemoveWidget "/Game/OpenMoba/Blueprints/Widgets/ScoreboardWidget.ScoreboardWidget_C")
          (else
            (CallFunction|AddWidget "/Game/OpenMoba/Blueprints/Widgets/ScoreboardWidget.ScoreboardWidget_C" 2)))))))

(event Input|ActionEvents|InputActionShop
  (params (Key :type Key%20Structure))
  ;[1 1 1] Shop
  (:Pressed
    (CallFunction|OpenShopWidget)))

(event Input|ActionEvents|InputActionRightMouseButtonDown
  (params (Key :type Key%20Structure))
  (bind (_worldlocation _worlddirection) (Game|Player|ConvertMouseLocationToWorldSpace))
  (bind (_worldlocation_2 _worlddirection_2) (Game|Player|ConvertMouseLocationToWorldSpace))
  ;[1 1 1] RightMouseButtonDown
  (:Pressed
    (if (Utilities|IsCommandUnitValid)
      (bind _outhits (Collision|MultiLineTraceByChannel _worldlocation (+ _worldlocation (* _worlddirection 1e+04)) "TraceTypeQuery4" false 0 "None"))
      (Variables|Client|SetAttackUnit false)
      (bind _array_element (Utilities|Array|ForEachLoopwithBreak _outhits :!label _label)
        (:LoopBody
          (bind _asunit (Utilities|Casting|CastToUnit (.HitActor (Collision|BreakHitResult _array_element))))
          (bind _alive (Default|IsAlive _asunit))
          (bind _asmy_player_state (Utilities|Casting|CastToMyPlayerState (Variables|GetPlayerState)))
          (bind _vision (Default|GetVision _asunit (Variables|/Game/OpenMoba/Blueprints/PlayerState/MyPlayerState.MyPlayerState_C|GetTeam _asmy_player_state)))
          (if (Math|Boolean|ANDBoolean (Utilities|Enum|NotEqual(Enum) _vision "NewEnumerator2") (Utilities|Enum|NotEqual(Enum) (Variables|/Game/OpenMoba/Blueprints/PlayerState/MyPlayerState.MyPlayerState_C|GetTeam _asmy_player_state) (Variables|/Game/OpenMoba/Blueprints/Units/Unit.Unit_C|GetTeam _asunit)) _alive)
            (CallFunction|SendAttack _asunit)
            (Variables|Client|SetAttackUnit true)
            (goto _label Break)))
        (:Completed
          (if (not (Variables|Client|GetAttackUnit))
            (bind (_outhit _returnvalue) (Collision|LineTraceByChannel _worldlocation_2 (+ _worldlocation_2 (* _worlddirection_2 1e+04)) "TraceTypeQuery3" false 0 "None"))
            (if _returnvalue
              (CallFunction|SendMoveCommand (.Location (Collision|BreakHitResult _outhit))))))))))

(event Input|ActionEvents|InputActionConsumeItem1
  (params (Key :type Key%20Structure))
  ;[1 1 1] ConsumeItem
  (:Pressed
    (CallFunction|SendConsumeItem 1)))

(event Input|ActionEvents|InputActionConsumeItem2
  (params (Key :type Key%20Structure))
  ;[1 1 1] ConsumeItem
  (:Pressed
    (CallFunction|SendConsumeItem 2)))

(event Input|ActionEvents|InputActionConsumeItem3
  (params (Key :type Key%20Structure))
  ;[1 1 1] ConsumeItem
  (:Pressed
    (CallFunction|SendConsumeItem 3)))

(event Input|ActionEvents|InputActionConsumeItem4
  (params (Key :type Key%20Structure))
  ;[1 1 1] ConsumeItem
  (:Pressed
    (CallFunction|SendConsumeItem 4)))

(event Input|ActionEvents|InputActionConsumeItem5
  (params (Key :type Key%20Structure))
  ;[1 1 1] ConsumeItem
  (:Pressed
    (CallFunction|SendConsumeItem 5)))

(event Custom|CreateCamera
  (bind _commandunit (Variables|Client&Server|GetCommandUnit))
  ;[1 1 1] CreateCamera
  (Utilities|IsValid _commandunit
    (:Is%20Valid
      (if (not (Utilities|IsValid (Variables|Client|GetClientCamera)))
        (bind _returnvalue (Game|SpawnActorfromClass "/Game/OpenMoba/Blueprints/Camera/ClientCamera.ClientCamera_C" (Math|Transform|MakeTransform (Transformation|GetActorLocation _commandunit)) "AlwaysSpawn" 0 0))
        (bind _output_get (Variables|Client|SetClientCamera _returnvalue)))
      (Default|Init _output_get (Variables|Client&Server|GetCommandUnit)))))

(event Custom|ScrollCamera
  ;[1 1 1] Tick
  (Utilities|IsValid (Variables|Client|GetClientCamera)
    (:Is%20Valid
      (Utilities|FlowControl|Sequence
        (:then_0
          (if (Game|Player|IsInputKeyDown (Variables|Client|GetScrollUpKey))
            (Default|Scroll (Variables|Client|GetClientCamera) "1000.000000, 0, 0")
            (elif (Game|Player|IsInputKeyDown (Variables|Client|GetScrollDownKey))
              (Default|Scroll (Variables|Client|GetClientCamera) "-1000.000000, 0, 0"))))
        (:then_1
          (if (Game|Player|IsInputKeyDown (Variables|Client|GetScrollRightKey))
            (Default|Scroll (Variables|Client|GetClientCamera) "0.000000,1000.000000, 0")
            (elif (Game|Player|IsInputKeyDown (Variables|Client|GetScrollLeftKey))
              (Default|Scroll (Variables|Client|GetClientCamera) "0.000000,-1000.000000, 0"))))))))

(event Input|ActionEvents|InputActionAutoFollow
  (params (Key :type Key%20Structure))
  (bind _clientcamera (Variables|Client|GetClientCamera))
  ;[1 1 1] AutoFollow
  (:Pressed
    (Utilities|IsValid _clientcamera
      (:Is%20Valid
        (Default|AutoFollowActor _clientcamera)))))

(event Input|ActionEvents|InputActionZoomIn
  (params (Key :type Key%20Structure))
  (bind _clientcamera (Variables|Client|GetClientCamera))
  (:Pressed
    (Utilities|IsValid _clientcamera
      (:Is%20Valid
        (Default|Zoom _clientcamera 1.0)))))

(event Input|ActionEvents|InputActionZoomOut
  (params (Key :type Key%20Structure))
  (bind _clientcamera (Variables|Client|GetClientCamera))
  (:Pressed
    (Utilities|IsValid _clientcamera
      (:Is%20Valid
        (Default|Zoom _clientcamera -1.0)))))

(event EventRemoveWidget
  (params (Class :type User%20Widget%20Class%20Reference))
  ;[1 1 1] RemoveWidget
  (bind _newparam (Utilities|GetMyGameInstance)
    (:Get
      (Default|RemoveWidget _newparam Class))))

(fn ConstructionScript)

(fn OnRepCommandUnit
  (if (Pawn|IsLocalPlayerController)
    (CallFunction|CreateCamera)))

(fn AddWidget
  (params (Class :type User%20Widget%20Class%20Reference) (ZOrder :type Integer))
  (bind _newparam (Utilities|GetMyGameInstance)
    (:Get
      (bind _widget (Default|AddWidget _newparam Class ZOrder))
      (return _widget))))

(fn GetWidget
  (params (Class :type User%20Widget%20Class%20Reference))
  (bind _newparam (Utilities|GetMyGameInstance)
    (:Get
      (bind _widget (Default|GetWidget _newparam Class))
      (return _widget))))

(fn IsWidgetVisible
  (params (Class :type User%20Widget%20Class%20Reference))
  (bind _newparam (Utilities|GetMyGameInstance)
    (:Get
      (bind (_visible _widget) (Default|IsWidgetVisible _newparam Class))
      (return _visible _widget))))